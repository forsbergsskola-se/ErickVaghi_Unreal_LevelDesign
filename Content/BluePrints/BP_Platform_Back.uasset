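; BP_Platform_Back is a platform actor that shuttles back and forth once its Movement event receives Open as true.
; A timeline drives Alpha, applying the Move function's location and rotation outputs to Platform each update.
; On finish it waits for Pause, then a FlipFlop alternates reverse and play.
; Move holds lerps between initial transform and Destination offset, shown unconnected, with rotation endpoints ordered opposite to location.
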(event `self.Movement`
  (params (Open :type Boolean))
  (bind (_newparam _newparam2) (`self.Move` (`self.InitPos`) (`self.InitRot`) (`self.Destination`)))
  (if Open
    (bind (_direction _alpha) (`Timeline|Timeline_0` :!label _label)
      (:`Update`
        (set `self.Alpha` _alpha)
        (`SceneComponent.K2_SetRelativeLocationAndRotation` (`self.Platform`) _newparam _newparam2 false false))
      (:`Finished`
        (`KismetSystemLibrary.Delay` (`self.Pause`))
        (`/Engine/EditorBlueprintResources/StandardMacros.FlipFlop`
          (:`A`
            (goto _label :!via `Reverse`))
          (:`B`
            (goto _label)))))))

(fn `UserConstructionScript`
  (`parent.UserConstructionScript`))