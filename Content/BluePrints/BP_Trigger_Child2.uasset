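; BP_Trigger_Child2 is a trigger child Blueprint that acts as an open/close toggle for a moving platform, with indicator lights.
; Its MovePlatform event uses a FlipFlop to alternate Light and Light1 between green and red emissive materials, set Open true or false, and pass that state through CallMovePlatform.
; The construction script defers to the parent, and BeginPlay, overlap and Tick are disabled stubs.
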(event `self.Move Platform`
  (`/Engine/EditorBlueprintResources/StandardMacros.FlipFlop`
    (:`A`
      (`PrimitiveComponent.SetMaterial` (`self.Light1`) 0 (`self.Green_Emission`))
      (`PrimitiveComponent.SetMaterial` (`self.Light`) 0 (`self.Green_Emission`))
      (bind _output_get (set `self.Open` true))
      (`self.Move_Platform` _output_get))
    (:`B`
      (`PrimitiveComponent.SetMaterial` (`self.Light1`) 0 (`self.Red_Emission`))
      (`PrimitiveComponent.SetMaterial` (`self.Light`) 0 (`self.Red_Emission`))
      (bind _output_get_2 (set `self.Open` false))
      (`self.Move_Platform` _output_get_2))))

(fn `UserConstructionScript`
  (`parent.UserConstructionScript`))