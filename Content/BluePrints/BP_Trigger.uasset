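; BP_Trigger is an interaction switch that toggles an Open state to drive a platform.
; Entering its collider shows an Interract prompt widget and binds MovePlatform to the BP_FP_Character's PushInteraction; leaving removes all widgets and unbinds it.
; Each interaction flips Open through a FlipFlop, swaps the Light material between green and red emission, and passes the state out through CallMovePlatform.
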(event `self.Collider.OnComponentBeginOverlap`
  (params (OverlappedComponent :type "PrimitiveComponent Object Reference") (OtherActor :type "Actor Object Reference") (OtherComp :type "PrimitiveComponent Object Reference") (OtherBodyIndex :type Integer) (bFromSweep :type Boolean) (SweepResult :type "HitResult Structure (by ref)"))
  ;[1 1 1] Enter Trigger
  ;;[1 1 1] Show instructions
  (bind _returnvalue (`|CreateWidget` "/Game/Widgets/Interract.Interract_C"))
  (bind _output_get (set `self.NewVar_1` _returnvalue))
  (`UserWidget.AddToViewport` _output_get 0)
  (bind _asbp_fp_character (cast `/Game/FirstPerson/Blueprints/BP_FP_Character` OtherActor))
  (add `/Game/FirstPerson/Blueprints/BP_FP_Character.Push_Interaction` _asbp_fp_character (delegate `Move Platform`)))

(event `Move Platform`
  (`/Engine/EditorBlueprintResources/StandardMacros.FlipFlop`
    (:`A`
      (`PrimitiveComponent.SetMaterial` (`self.Light`) 0 (`self.Green_Emission`))
      (bind _output_get (set `self.Open` true))
      (`self.Move_Platform` _output_get))
    (:`B`
      (`PrimitiveComponent.SetMaterial` (`self.Light`) 0 (`self.Red_Emission`))
      (bind _output_get_2 (set `self.Open` false))
      (`self.Move_Platform` _output_get_2))))

(event `self.ReceiveBeginPlay`
  ;[1 1 1] Set Door closed
  (set `self.Open` false))

(event `self.Collider.OnComponentEndOverlap`
  (params (OverlappedComponent :type "PrimitiveComponent Object Reference") (OtherActor :type "Actor Object Reference") (OtherComp :type "PrimitiveComponent Object Reference") (OtherBodyIndex :type Integer))
  ;[1 1 1] Exit Trigger
  (`WidgetLayoutLibrary.RemoveAllWidgets`)
  (bind _asbp_fp_character (cast `/Game/FirstPerson/Blueprints/BP_FP_Character` OtherActor))
  (remove `/Game/FirstPerson/Blueprints/BP_FP_Character.Push_Interaction` _asbp_fp_character (delegate `Move Platform`)))

(fn `UserConstructionScript`)