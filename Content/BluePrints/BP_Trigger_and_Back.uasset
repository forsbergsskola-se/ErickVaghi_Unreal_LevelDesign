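; BP_Trigger_and_Back is a one-shot trigger that signals a platform to move.
; Its MovePlatform event switches the Light component to a green emissive material, destroys the Collider so it cannot be reused, sets Open to true and calls MovePlatform with that flag.
; Overlap and Tick are unused, so the event relies on being invoked from outside this graph.
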(event `self.Move Platform`
  (`PrimitiveComponent.SetMaterial` (`self.Light`) 0 (`self.Green_Emission`))
  (`ActorComponent.K2_DestroyComponent` (`self.Collider`))
  (bind _output_get (set `self.Open` true))
  (`self.Move_Platform` _output_get))

(fn `UserConstructionScript`
  (`parent.UserConstructionScript`))