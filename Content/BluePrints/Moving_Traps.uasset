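; Moving trap actor that animates its Trap component when triggered and reloads FirstPersonMap when BP_FP_Character overlaps it.
; BeginPlay stores the initial relative transform and binds MoveTrap to the Trigger's TrapActivated event.
; A timeline updates Alfa and applies the Move helper's outputs as relative location and rotation.
; Move contains lerps toward the Destination offset, shown unconnected, with the rotation lerp running in reverse.
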(event `self.ReceiveBeginPlay`
  (bind (_returnvalue_location _returnvalue_rotation) (`KismetMathLibrary.BreakTransform` (`SceneComponent.GetRelativeTransform` (`self.Trap`))))
  (set `self.InitPos` _returnvalue_location)
  (set `self.InitRot` _returnvalue_rotation)
  (add `/Game/BluePrints/Trap_Trigger.Trap_Activated` (`self.Trigger`) (delegate `MoveTrap`)))

(event `MoveTrap`
  (bind (_newparam _newparam2) (`self.Move` (`self.InitPos`) (`self.InitRot`) (`self.Destination`)))
  (bind (_direction _alpha) (`Timeline|Timeline_0`)
    (:`Update`
      (set `self.Alfa` _alpha)
      (`SceneComponent.K2_SetRelativeLocationAndRotation` (`self.Trap`) _newparam _newparam2 false false))))

(event `self.ReceiveActorBeginOverlap`
  (params (OtherActor :type "Actor Object Reference"))
  (cast `/Game/FirstPerson/Blueprints/BP_FP_Character` OtherActor)
  (`GameplayStatics.OpenLevelBySoftObjectPtr` "/Game/FirstPerson/Maps/FirstPersonMap.FirstPersonMap"))

(fn `UserConstructionScript`)