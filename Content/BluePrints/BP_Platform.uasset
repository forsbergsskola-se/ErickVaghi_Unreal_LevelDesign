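; BP_Platform is a platform that moves and rotates between its starting relative transform and a Destination offset when its Trigger signals it.
; BeginPlay caches the start transform and binds Movement to the Trigger's MovePlatform event.
; Movement plays or reverses the Animator timeline, whose Alpha drives the platform's location and rotation through the Move helper.
; Move's rotation lerp has its endpoints in reverse order to the location lerp.
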(event `self.ReceiveBeginPlay`
  (bind (_returnvalue_location _returnvalue_rotation) (`KismetMathLibrary.BreakTransform` (`SceneComponent.GetRelativeTransform` (`self.Platform`))))
  ;[1 1 1] Set Initial position
  (set `self.InitPos` _returnvalue_location)
  (set `self.InitRot` _returnvalue_rotation)
  ;[1 1 1] Get Input
  (add `/Game/BluePrints/BP_Trigger.Move_Platform` (`self.Trigger`) (delegate `Movement`)))

(event `Movement`
  (params (Open :type Boolean))
  (bind (_returnvalue _returnvalue2) (`self.Move` (`self.InitPos`) (`self.InitRot`) (`self.Destination`)))
  (if Open
    ;[1 1 1] Interpolate and Move
    (bind (_direction _alpha) (`Timeline|Animator` :!label _label)
      (:`Update`
        (set `self.Alpha` _alpha)
        (`SceneComponent.K2_SetRelativeLocationAndRotation` (`self.Platform`) _returnvalue _returnvalue2 false false)))
    (else
      (goto _label :!via `Reverse`))))

(fn `UserConstructionScript`)